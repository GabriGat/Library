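; Procedural bookcase actor that builds stacked shelves filled with books in its Construction Script.
; It reads shelf dimensions from a data table, adds one shelf mesh per level and fills every shelf above the bottom one.
; ShelfMode selects one repeated book with random depth misalignment or random books from a table.
; Books are placed side by side by table size until the width or book limit is reached.
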(event EventBeginPlay)

(event Collision|EventActorBeginOverlap
  (params (OtherActor :type Actor%20Object%20Reference)))

(event EventTick
  (params (DeltaSeconds :type Float%20%28single-precision%29)))

(fn ConstructionScript
  (CallFunction|CalculateDataOfShelf)
  (CallFunction|CreateBookcase))

(fn CreateShelf
  (params (Pivot :type Transform))
  ;[1 1 1] Piano
  (bind _returnvalue (AddComponent|AddStaticMeshComponent false (Math|Transform|MakeTransform (.location Pivot) "0, 0, 0" "1.000000,1.000000,1.000000")))
  (Components|StaticMesh|SetStaticMesh _returnvalue (Variables|Shelf|GetShelfMesh))
  (return))

(fn CreateBookcase
  (bind _height (Variables|PrivateShelf|GetHeight))
  ;[1 1 1] Loop  per la costruzione degli scaffali
  (for _index (range 0 (- (Variables|Shelf|GetShelvesNumber) 1))
    ;[1 1 1] Crea lo scaffale
    (CallFunction|CreateShelf (Math|Transform|MakeTransform (Math|Vector|MakeVector 0.0 0.0 (+ (* _index _height) (/ _height 2.0)))))
    ;[1 1 1] Controlla se é allo scaffale 0, se si non popolarlo
    (if (> _index 0)
      ;[1 1 1] Sceglie come popolare la libreria
      (switch int (Variables|Shelf|GetShelfMode)
        (:Default)
        (:0
          ;[1 1 1] Popola lo scaffale con un solo libro
          (CallFunction|CreateBooks (Math|Transform|MakeTransform (Math|Vector|MakeVector 0.0 0.0 (+ (* _index _height) (/ _height 2.0))))))
        (:1
          ;[1 1 1] Popola lo scaffale random
          (CallFunction|CreateBooksRandom (Math|Transform|MakeTransform (Math|Vector|MakeVector 0.0 0.0 (+ (* _index _height) (/ _height 2.0)))))))))
  (return))

(fn CreateBooksRandom
  (params (Pivot :type Transform))
  ;[1 1 1] Input
  ;[1 1 1] Calcola le posizioni iniziale del libro sullo scafale
  (bind _output_get (LocalVariables|SetBookStartPosition (- (/ (Variables|PrivateShelf|GetWidth) 2.0) (Variables|PrivateShelf|GetShelfThickShoulder))))
  (LocalVariables|SetBookActualPosition _output_get)
  ;[1 1 1] Calcola la posizione finale
  (LocalVariables|SetBookStopPosition (+ (/ (Variables|PrivateShelf|GetWidth) -2.0) (Variables|PrivateShelf|GetShelfThickShoulder)))
  ;[1 1 1] Inizializza il contatore di libri
  (LocalVariables|SetBooksNumber (Variables|Books|GetMaximumNumberOfBooks))
  ;[1 1 1] Loop di per la generazione dei libri
  (while (and (> (LocalVariables|GetBooksNumber) 0) (>= (LocalVariables|GetBookActualPosition) (LocalVariables|GetBookStopPosition)))
    ;[1 1 1] Recupera i dati del libro dalla tabella
    (bind _outrownames (DataTable|GetDataTableRowNames "/Game/Library/Asset3D/Book/S_TableBook.S_TableBook"))
    (bind _returnvalue (Utilities|GetDataTableRow "/Game/Library/Asset3D/Book/S_TableBook.S_TableBook" (.OutItem (Utilities|Array|Random _outrownames)))
      (:then
        ;[1 1 1] Calcola la posizione finale del libro
        (LocalVariables|SetBookActualPositionNext (Utilities|Operators|Subtract (LocalVariables|GetBookActualPosition) (.SizeDepth (Utilities|Struct|BreakS_Books _returnvalue))))
        ;[1 1 1] Aggiorna il contatore di libri
        (LocalVariables|SetBooksNumber (- (LocalVariables|GetBooksNumber) 1))
        ;[1 1 1] Verifica se il libro può essere contunuto nello scafale
        (if (>= (LocalVariables|GetBookActualPositionNext) (LocalVariables|GetBookStopPosition))
          ;[1 1 1] Genera il libro
          (bind _returnvalue_2 (AddComponent|AddStaticMeshComponent false (Math|Transform|MakeTransform (+ (Math|Vector|MakeVector (.TraLocX (Utilities|Struct|BreakS_Books _returnvalue)) (.TraLocY (Utilities|Struct|BreakS_Books _returnvalue)) (.TraLocZ (Utilities|Struct|BreakS_Books _returnvalue))) (Math|Vector|MakeVector 0.0 (LocalVariables|GetBookActualPosition) (+ (/ (Variables|PrivateShelf|GetHeight) -2.0) (/ (.SizeHeight (Utilities|Struct|BreakS_Books _returnvalue)) 2.0))) (.location Pivot)) (Math|Rotator|MakeRotator (.x (Math|Vector|MakeVector (.TraRotX (Utilities|Struct|BreakS_Books _returnvalue)) (.TraRotY (Utilities|Struct|BreakS_Books _returnvalue)) (.TraRotZ (Utilities|Struct|BreakS_Books _returnvalue)))) (.y (Math|Vector|MakeVector (.TraRotX (Utilities|Struct|BreakS_Books _returnvalue)) (.TraRotY (Utilities|Struct|BreakS_Books _returnvalue)) (.TraRotZ (Utilities|Struct|BreakS_Books _returnvalue)))) (.z (Math|Vector|MakeVector (.TraRotX (Utilities|Struct|BreakS_Books _returnvalue)) (.TraRotY (Utilities|Struct|BreakS_Books _returnvalue)) (.TraRotZ (Utilities|Struct|BreakS_Books _returnvalue))))))))
          (Components|StaticMesh|SetStaticMesh _returnvalue_2 (.RefBook (Utilities|Struct|BreakS_Books _returnvalue)))
          ;[1 1 1] Aggiorn BookActualPosition e BookActualPositionNext
          (LocalVariables|SetBookActualPosition (LocalVariables|GetBookActualPositionNext))
          (else
            (return true))))
      (:RowNotFound
        (return false))))
  (return true))

(fn CalculateDataOfShelf
  ;[1 1 1] Recupera i dati dello scaffale dalla tabella
  (bind _returnvalue (Utilities|GetDataTableRow (Variables|Shelf|GetShelfSize) "Size")
    (:then
      ;[1 1 1] Inizializza le variabili dello scaffale
      (Variables|PrivateShelf|SetShelfWidth (.Width (Utilities|Struct|BreakS_Shelf _returnvalue)))
      (Variables|PrivateShelf|SetShelfHeight (.Hight (Utilities|Struct|BreakS_Shelf _returnvalue)))
      (Variables|PrivateShelf|SetShelfDepth (.Depth (Utilities|Struct|BreakS_Shelf _returnvalue)))
      (Variables|PrivateShelf|SetShelfThickShoulder (.ThickShoulder (Utilities|Struct|BreakS_Shelf _returnvalue)))
      (Variables|PrivateShelf|SetShelfTopThickness (.TopThickness (Utilities|Struct|BreakS_Shelf _returnvalue)))
      (Variables|PrivateShelf|SetWidth (Variables|PrivateShelf|GetShelfWidth))
      (Variables|PrivateShelf|SetHeight (Variables|PrivateShelf|GetShelfHeight))
      (Variables|PrivateShelf|SetDepth (Variables|PrivateShelf|GetShelfDepth))
      (return))))

(fn CreateBooks
  (params (Pivot :type Transform))
  (bind _disalineamentrandombooks (Variables|Books|GetDisalineamentRandomBooks))
  ;[1 1 1] Input
  ;[1 1 1] Calcola le posizioni iniziale del libro sullo scafale
  (bind _output_get (LocalVariables|SetBookStartPosition (- (/ (Variables|PrivateShelf|GetWidth) 2.0) (Variables|PrivateShelf|GetShelfThickShoulder))))
  (LocalVariables|SetBookActualPosition _output_get)
  ;[1 1 1] Calcola la posizione finale
  (LocalVariables|SetBookStopPosition (+ (/ (Variables|PrivateShelf|GetWidth) -2.0) (Variables|PrivateShelf|GetShelfThickShoulder)))
  ;[1 1 1] Inizializza il contatore di libri
  (LocalVariables|SetBooksNumber (Variables|Books|GetMaximumNumberOfBooks))
  ;[1 1 1] Loop di per la generazione dei libri
  (while (and (> (LocalVariables|GetBooksNumber) 0) (>= (LocalVariables|GetBookActualPosition) (LocalVariables|GetBookStopPosition)))
    ;[1 1 1] Recupera i dati del libro dalla tabella
    (bind _outrownames (DataTable|GetDataTableRowNames "/Game/Library/Asset3D/Book/S_TableBook.S_TableBook"))
    (bind _returnvalue (Utilities|GetDataTableRow "/Game/Library/Asset3D/Book/S_TableBook.S_TableBook" (Utilities|Array|Get(acopy) _outrownames (- (Variables|Books|GetSingleBook) 1)))
      (:then
        ;[1 1 1] Calcola la posizione finale del libro
        (LocalVariables|SetBookActualPositionNext (Utilities|Operators|Subtract (LocalVariables|GetBookActualPosition) (.SizeDepth (Utilities|Struct|BreakS_Books _returnvalue))))
        ;[1 1 1] Aggiorna il contatore di libri
        (LocalVariables|SetBooksNumber (- (LocalVariables|GetBooksNumber) 1))
        ;[1 1 1] Verifica se il libro può essere contunuto nello scafale
        (if (>= (LocalVariables|GetBookActualPositionNext) (LocalVariables|GetBookStopPosition))
          ;[1 1 1] Genera il libro
          (bind _returnvalue_2 (AddComponent|AddStaticMeshComponent false (Math|Transform|MakeTransform (+ (Math|Vector|MakeVector (.TraLocX (Utilities|Struct|BreakS_Books _returnvalue)) (.TraLocY (Utilities|Struct|BreakS_Books _returnvalue)) (.TraLocZ (Utilities|Struct|BreakS_Books _returnvalue))) (Math|Vector|MakeVector (Math|Random|RandomFloatinRange (* _disalineamentrandombooks -1.0) _disalineamentrandombooks) (LocalVariables|GetBookActualPosition) (+ (/ (Variables|PrivateShelf|GetHeight) -2.0) (/ (.SizeHeight (Utilities|Struct|BreakS_Books _returnvalue)) 2.0))) (.location Pivot)) (Math|Rotator|MakeRotator (.x (Math|Vector|MakeVector (.TraRotX (Utilities|Struct|BreakS_Books _returnvalue)) (.TraRotY (Utilities|Struct|BreakS_Books _returnvalue)) (.TraRotZ (Utilities|Struct|BreakS_Books _returnvalue)))) (.y (Math|Vector|MakeVector (.TraRotX (Utilities|Struct|BreakS_Books _returnvalue)) (.TraRotY (Utilities|Struct|BreakS_Books _returnvalue)) (.TraRotZ (Utilities|Struct|BreakS_Books _returnvalue)))) (.z (Math|Vector|MakeVector (.TraRotX (Utilities|Struct|BreakS_Books _returnvalue)) (.TraRotY (Utilities|Struct|BreakS_Books _returnvalue)) (.TraRotZ (Utilities|Struct|BreakS_Books _returnvalue))))))))
          (Components|StaticMesh|SetStaticMesh _returnvalue_2 (.RefBook (Utilities|Struct|BreakS_Books _returnvalue)))
          ;[1 1 1] Aggiorn BookActualPosition e BookActualPositionNext
          (LocalVariables|SetBookActualPosition (LocalVariables|GetBookActualPositionNext))
          (else
            (return true))))
      (:RowNotFound
        (return false))))
  (return true))