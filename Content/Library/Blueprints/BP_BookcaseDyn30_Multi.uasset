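; Bookcase Blueprint that procedurally builds a row of NumberOfLibraries bookcases for a library scene.
; The Construction Script runs InitObject and CalculateDataOfShelfDyn, then CreateLibrary, bypassing the parent construction script.
; CreateLibrary calls CreateBookcase per unit, stepping by Width along Y from the pivot location with fixed zero rotation and unit scale.
; It has no active runtime event logic.
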(event EventBeginPlay
  (|CallParentFunction) ; This node is disabled and will not be called.\nDrag off pins to build functionality.
)

(event Collision|EventActorBeginOverlap
  (params (OtherActor :type Actor%20Object%20Reference))
  (|CallParentFunction OtherActor) ; This node is disabled and will not be called.\nDrag off pins to build functionality.
)

(event EventTick
  (params (DeltaSeconds :type Float%20%28single-precision%29))
  (|CallParentFunction DeltaSeconds) ; This node is disabled and will not be called.\nDrag off pins to build functionality.
)

(fn ConstructionScript
  (if true
    (CallFunction|InitObject)
    (CallFunction|CalculateDataOfShelfDyn)
    (CallFunction|CreateLibrary)
    (else
      (|CallParentFunction))))

(fn CreateLibrary
  (params (Pivot :type Transform) (Pivot_Location :type Vector :default "0, 0, 0") (Pivot_Rotation :type Rotator :default "0, 0, 0") (Pivot_Scale :type Vector :default "0, 0, 0"))
  ;[1 1 1] Loop  per la costruzione delle librerie
  (for _index (range 0 (- (Variables|Shelf|GetNumberOfLibraries) 1))
    ;[1 1 1] Crea Bookcase
    (CallFunction|CreateBookcase (Math|Transform|MakeTransform (+ (Math|Vector|MakeVector 0.0 (* _index (Variables|Default|GetWidth)) 0.0) (.location Pivot)))))
  (return))