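; Procedural bookcase actor that builds a stack of shelves and fills them with books in the construction script.
; Scaled width, height and depth drive a shelf loop, each level adding a board and two side panels from the ShelfType mesh.
; Every level except the top gets books from the S_TableBook data table, either repeated Book01 or random rows with per-book offsets, chosen by ShelfMode.
; Books advance across the width by their depth until the next would overflow.
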(event EventBeginPlay)

(event Collision|EventActorBeginOverlap
  (params (OtherActor :type Actor%20Object%20Reference)))

(event EventTick
  (params (DeltaSeconds :type Float%20%28single-precision%29)))

(fn ConstructionScript
  ;[1 1 1] Calcola le dimensioni reali
  (Variables|Size|SetWidth (* (Variables|Size|GetWidthS1) (Variables|Scale|GetScaleWidth)))
  (Variables|Size|SetHeight (* (Variables|Size|GetHeightS1) (Variables|Scale|GetScaleHeight)))
  (Variables|Size|SetDepth (* (Variables|Size|GetDepthS1) (Variables|Scale|GetScaleDepth)))
  (CallFunction|CreateBookcase))

(fn CreateShelf
  (params (Pivot :type Transform))
  (bind _returnvalue (Math|Vector|MakeVector 1.95 0.81 1.0))
  (bind _returnvalue_2 (Math|Vector|MakeVector 0.63 0.81 1.0))
  (bind _widths1 (Variables|Size|GetWidthS1))
  (bind _thicknesss1 (Variables|Size|GetThicknessS1))
  (bind _heights1 (Variables|Size|GetHeightS1))
  (bind _scaleheight (Variables|Scale|GetScaleHeight))
  (bind _scaledepth (Variables|Scale|GetScaleDepth))
  (bind _scalewidth (Variables|Scale|GetScaleWidth))
  (bind _scaleheight_2 (Variables|Scale|GetScaleHeight))
  (bind _scaleheight_3 (Variables|Scale|GetScaleHeight))
  (bind _thicknesss1_2 (Variables|Size|GetThicknessS1))
  (bind _returnvalue_3 (/ _widths1 2.0))
  (bind _returnvalue_4 (/ _thicknesss1_2 2.0))
  (bind _returnvalue_5 (* _scaleheight_2 (.x _returnvalue_2)))
  (bind _returnvalue_6 (/ _heights1 -2.0))
  (bind _returnvalue_7 (/ _thicknesss1 2.0))
  (bind _returnvalue_8 (* (.y _returnvalue_2) _scaledepth))
  (bind _returnvalue_9 (Math|Vector|MakeVector _returnvalue_5 _returnvalue_8 1.0))
  (bind _returnvalue_10 (* _returnvalue_3 _scalewidth))
  (bind _returnvalue_11 (* _scaleheight _returnvalue_6))
  (bind _returnvalue_12 (* _returnvalue_7 _scaleheight_3 -1.0))
  (bind _returnvalue_13 (- _returnvalue_10 _returnvalue_4))
  (bind _returnvalue_14 (Utilities|Operators|Subtract _returnvalue_11 _returnvalue_7 _returnvalue_12))
  ;[1 1 1] Piano
  (bind _returnvalue_15 (AddComponent|AddStaticMeshComponent false (Math|Transform|MakeTransform (.location Pivot) "0,90.000000, 0" (Math|Vector|MakeVector (* (Variables|Scale|GetScaleWidth) (.x _returnvalue)) (* (Variables|Scale|GetScaleDepth) (.y _returnvalue)) (.z _returnvalue)))))
  (Components|StaticMesh|SetStaticMesh _returnvalue_15 (Variables|Shelf|GetShelfType))
  ;[1 1 1] Spalla sx
  (bind _returnvalue_16 (AddComponent|AddStaticMeshComponent false (Math|Transform|MakeTransform (+ (.location Pivot) (Math|Vector|MakeVector 0.0 _returnvalue_13 _returnvalue_14)) "90.000000,90.000000, 0" _returnvalue_9)))
  (Components|StaticMesh|SetStaticMesh _returnvalue_16 (Variables|Shelf|GetShelfType))
  ;[1 1 1] Spalla dx
  (bind _returnvalue_17 (AddComponent|AddStaticMeshComponent false (Math|Transform|MakeTransform (+ (.location Pivot) (Math|Vector|MakeVector 0.0 (* _returnvalue_13 -1.0) _returnvalue_14)) "90.000000,90.000000, 0" _returnvalue_9)))
  (Components|StaticMesh|SetStaticMesh _returnvalue_17 (Variables|Shelf|GetShelfType))
  (return))

(fn CreateBookcase
  ;[1 1 1] Loop  per la costruzione degli scaffali
  (for _index (range 0 (- (Variables|Shelf|Get%20ShelvesNumber) 1))
    ;[1 1 1] Crea lo scaffale
    (CallFunction|CreateShelf (Math|Transform|MakeTransform (Math|Vector|MakeVector 0.0 0.0 (* _index (Variables|Size|GetHeight)))))
    ;[1 1 1] Controlla se é arrivato all' ultimo scaffale
    (if (< _index (- (Variables|Shelf|Get%20ShelvesNumber) 1))
      ;[1 1 1] Sceglie come popolare la libreria
      (switch int (Variables|Shelf|GetShelfMode)
        (:Default)
        (:0
          ;[1 1 1] Popola lo scaffale con un solo libro
          (CallFunction|CreateBooks (Math|Transform|MakeTransform (Math|Vector|MakeVector 0.0 0.0 (* _index (Variables|Size|GetHeight))))))
        (:1
          ;[1 1 1] Popola lo scaffale random
          (CallFunction|CreateBooksRandom (Math|Transform|MakeTransform (Math|Vector|MakeVector 0.0 0.0 (* _index (Variables|Size|GetHeight)))))))))
  (return))

(fn CreateBooks
  (params (Pivot :type Transform))
  ;[1 1 1] Input
  ;[1 1 1] Calcola le posizioni iniziale del libro sullo scafale
  (bind _output_get (LocalVariables|SetBookStartPosition (- (/ (Variables|Size|GetWidth) 2.0) (Variables|Size|GetThicknessS1))))
  (bind _output_get_2 (LocalVariables|SetBookActualPosition _output_get))
  ;[1 1 1] Calcola la posizione del libro successivo
  (LocalVariables|SetBookActualPositionNext (- _output_get_2 (Variables|Size|GetThicknessS1)))
  ;[1 1 1] Calcola la posizione finale
  (LocalVariables|SetBookStopPosition (+ (/ (Variables|Size|GetWidth) -2.0) (Variables|Size|GetThicknessS1)))
  ;[1 1 1] Inizializza il contatore di libri
  (LocalVariables|SetBooksNumber 100)
  ;[1 1 1] Recupera i dati del libro dalla tabella
  (bind _returnvalue (Utilities|GetDataTableRow "/Game/Library/Asset3D/Book/S_TableBook.S_TableBook" "Book01")
    (:then
      ;[1 1 1] Loop di per la generazione dei libri
      (while (and (> (LocalVariables|GetBooksNumber) 0) (>= (LocalVariables|GetBookActualPosition) (LocalVariables|GetBookStopPosition)))
        ;[1 1 1] Aggiorna il contatore di libri
        (LocalVariables|SetBooksNumber (- (LocalVariables|GetBooksNumber) 1))
        ;[1 1 1] Verifica se il libro può essere contunuto nello scafale
        (if (>= (LocalVariables|GetBookActualPositionNext) (LocalVariables|GetBookStopPosition))
          ;[1 1 1] Genera il libro
          (bind _returnvalue_2 (AddComponent|AddStaticMeshComponent false (Math|Transform|MakeTransform (+ (Math|Vector|MakeVector 0.0 (LocalVariables|GetBookActualPosition) (/ (+ (Variables|Size|GetThicknessS1) (.SizeHeight (Utilities|Struct|BreakS_Books _returnvalue))) 2.0)) (.location Pivot)) "90.000000,90.000000, 0" "1.000000,1.000000,1.000000")))
          (Components|StaticMesh|SetStaticMesh _returnvalue_2 (.RefBook (Utilities|Struct|BreakS_Books _returnvalue)))
          ;[1 1 1] Aggiorn BookActualPosition e BookActualPositionNext
          (LocalVariables|SetBookActualPosition (LocalVariables|GetBookActualPositionNext))
          (LocalVariables|SetBookActualPositionNext (- (LocalVariables|GetBookActualPositionNext) (.SizeDepth (Utilities|Struct|BreakS_Books _returnvalue))))
          (else
            (return true))))
      (return true))
    (:RowNotFound
      (return false))))

(fn CreateBooksRandom
  (params (Pivot :type Transform))
  ;[1 1 1] Input
  ;[1 1 1] Calcola le posizioni iniziale del libro sullo scafale
  (bind _output_get (LocalVariables|SetBookStartPosition (- (/ (Variables|Size|GetWidth) 2.0) (Variables|Size|GetThicknessS1))))
  (LocalVariables|SetBookActualPosition _output_get)
  ;[1 1 1] Calcola la posizione finale
  (LocalVariables|SetBookStopPosition (+ (/ (Variables|Size|GetWidth) -2.0) (Variables|Size|GetThicknessS1)))
  ;[1 1 1] Inizializza il contatore di libri
  (LocalVariables|SetBooksNumber 100)
  ;[1 1 1] Loop di per la generazione dei libri
  (while (and (> (LocalVariables|GetBooksNumber) 0) (>= (LocalVariables|GetBookActualPosition) (LocalVariables|GetBookStopPosition)))
    ;[1 1 1] Recupera i dati del libro dalla tabella
    (bind _outrownames (DataTable|GetDataTableRowNames "/Game/Library/Asset3D/Book/S_TableBook.S_TableBook"))
    (bind _returnvalue (Utilities|GetDataTableRow "/Game/Library/Asset3D/Book/S_TableBook.S_TableBook" (.OutItem (Utilities|Array|Random _outrownames)))
      (:then
        ;[1 1 1] Calcola la posizione finale del libro
        (LocalVariables|SetBookActualPositionNext (Utilities|Operators|Subtract (LocalVariables|GetBookActualPosition) (.SizeDepth (Utilities|Struct|BreakS_Books _returnvalue))))
        ;[1 1 1] Aggiorna il contatore di libri
        (LocalVariables|SetBooksNumber (- (LocalVariables|GetBooksNumber) 1))
        ;[1 1 1] Verifica se il libro può essere contunuto nello scafale
        (if (>= (LocalVariables|GetBookActualPositionNext) (LocalVariables|GetBookStopPosition))
          ;[1 1 1] Genera il libro
          (bind _returnvalue_2 (AddComponent|AddStaticMeshComponent false (Math|Transform|MakeTransform (+ (Math|Vector|MakeVector (.TraLocX (Utilities|Struct|BreakS_Books _returnvalue)) (.TraLocY (Utilities|Struct|BreakS_Books _returnvalue)) (.TraLocZ (Utilities|Struct|BreakS_Books _returnvalue))) (Math|Vector|MakeVector 0.0 (LocalVariables|GetBookActualPosition) (/ (+ (.SizeHeight (Utilities|Struct|BreakS_Books _returnvalue)) (Variables|Size|GetThicknessS1)) 2.0)) (.location Pivot)) (Math|Rotator|MakeRotator (.x (Math|Vector|MakeVector (.TraRotX (Utilities|Struct|BreakS_Books _returnvalue)) (.TraRotY (Utilities|Struct|BreakS_Books _returnvalue)) (.TraRotZ (Utilities|Struct|BreakS_Books _returnvalue)))) (.y (Math|Vector|MakeVector (.TraRotX (Utilities|Struct|BreakS_Books _returnvalue)) (.TraRotY (Utilities|Struct|BreakS_Books _returnvalue)) (.TraRotZ (Utilities|Struct|BreakS_Books _returnvalue)))) (.z (Math|Vector|MakeVector (.TraRotX (Utilities|Struct|BreakS_Books _returnvalue)) (.TraRotY (Utilities|Struct|BreakS_Books _returnvalue)) (.TraRotZ (Utilities|Struct|BreakS_Books _returnvalue))))))))
          (Components|StaticMesh|SetStaticMesh _returnvalue_2 (.RefBook (Utilities|Struct|BreakS_Books _returnvalue)))
          ;[1 1 1] Aggiorn BookActualPosition e BookActualPositionNext
          (LocalVariables|SetBookActualPosition (LocalVariables|GetBookActualPositionNext))
          (else
            (return true))))
      (:RowNotFound
        (return false))))
  (return true))