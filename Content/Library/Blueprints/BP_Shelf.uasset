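; BP_Shelf is a parametric shelf that assembles itself in the Construction Script, with no runtime logic.
; It adds three instances of one Model mesh as components: a horizontal top board and two rotated side supports below it.
; Width, height and depth multipliers scale the base proportions, leaving board thickness unscaled.
; Support offsets derive from the base dimensions and thickness, keeping the sides inset at the board's ends as it resizes.
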(event EventBeginPlay)

(event Collision|EventActorBeginOverlap
  (params (OtherActor :type Actor%20Object%20Reference)))

(event EventTick
  (params (DeltaSeconds :type Float%20%28single-precision%29)))

(fn ConstructionScript
  (bind _returnvalue (Math|Vector|MakeVector 1.95 0.81 1.0))
  (bind _returnvalue_2 (Math|Vector|MakeVector 0.63 0.81 1.0))
  (bind _widths1 (Variables|Size|GetWidthS1))
  (bind _thicknesss1 (Variables|Size|GetThicknessS1))
  (bind _heights1 (Variables|Size|GetHeightS1))
  (bind _scaleheight (Variables|Scale|GetScaleHeight))
  (bind _scaledepth (Variables|Scale|GetScaleDepth))
  (bind _scalewidth (Variables|Scale|GetScaleWidth))
  (bind _scaleheight_2 (Variables|Scale|GetScaleHeight))
  (bind _scaleheight_3 (Variables|Scale|GetScaleHeight))
  (bind _thicknesss1_2 (Variables|Size|GetThicknessS1))
  (bind _returnvalue_3 (/ _widths1 2.0))
  (bind _returnvalue_4 (/ _thicknesss1_2 2.0))
  (bind _returnvalue_5 (* _scaleheight_2 (.x _returnvalue_2)))
  (bind _returnvalue_6 (/ _heights1 -2.0))
  (bind _returnvalue_7 (/ _thicknesss1 -2.0))
  (bind _returnvalue_8 (* (.y _returnvalue_2) _scaledepth))
  (bind _returnvalue_9 (- _scaleheight_3 1.0))
  (bind _returnvalue_10 (Math|Vector|MakeVector _returnvalue_5 _returnvalue_8 1.0))
  (bind _returnvalue_11 (* _returnvalue_3 _scalewidth))
  (bind _returnvalue_12 (* _scaleheight _returnvalue_6))
  (bind _returnvalue_13 (* _returnvalue_7 _returnvalue_9))
  (bind _returnvalue_14 (- _returnvalue_11 _returnvalue_4))
  (bind _returnvalue_15 (- _returnvalue_12 _returnvalue_13))
  ;[1 1 1] Piano
  (bind _returnvalue_16 (AddComponent|AddStaticMeshComponent false (Math|Transform|MakeTransform "0, 0, 0" "0,90.000000, 0" (Math|Vector|MakeVector (* (Variables|Scale|GetScaleWidth) (.x _returnvalue)) (* (Variables|Scale|GetScaleDepth) (.y _returnvalue)) (.z _returnvalue)))))
  (Components|StaticMesh|SetStaticMesh _returnvalue_16 (Variables|Model|GetModel))
  ;[1 1 1] Spalla sx
  (bind _returnvalue_17 (AddComponent|AddStaticMeshComponent false (Math|Transform|MakeTransform (Math|Vector|MakeVector 0.0 _returnvalue_14 _returnvalue_15) "90.000000,90.000000, 0" _returnvalue_10)))
  (Components|StaticMesh|SetStaticMesh _returnvalue_17 (Variables|Model|GetModel))
  ;[1 1 1] Spalla dx
  (bind _returnvalue_18 (AddComponent|AddStaticMeshComponent false (Math|Transform|MakeTransform (Math|Vector|MakeVector 0.0 (* _returnvalue_14 -1.0) _returnvalue_15) "90.000000,90.000000, 0" _returnvalue_10)))
  (Components|StaticMesh|SetStaticMesh _returnvalue_18 (Variables|Model|GetModel)))